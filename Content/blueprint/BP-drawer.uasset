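; Interactive drawer Blueprint that toggles a drawer mesh open or closed on the interact input.
; A 500-unit forward trace from the VR_Pawn finds the mesh, and its relative X selects the open or close branch.
; Each branch calls a sound, stores endpoints 30 units apart and plays a timeline.
; The endpoint lerps are unconnected, so both timeline updates set the mesh's relative location to zero.
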(event `self.ReceiveBeginPlay`
  (`self.EnableInput` (`GameplayStatics.GetPlayerController` 0) null))

(event `InputAction|interact`
  (params (Key :type "Key Structure"))
  (bind _returnvalue (`self.K2_GetActorLocation`))
  (bind (_relativelocation_x _relativelocation_y _relativelocation_z) (`KismetMathLibrary.BreakVector` (`SceneComponent.RelativeLocation` (`self.Static mesh REF`))))
  (bind (_relativelocation_x_2 _relativelocation_y_2 _relativelocation_z_2) (`KismetMathLibrary.BreakVector` (`SceneComponent.RelativeLocation` (`self.Static mesh REF`))))
  (:`Pressed`
    (bind _asvr_pawn (cast `/Game/VirtualRealityBP/Blueprints/VR_Pawn` (`GameplayStatics.GetPlayerCharacter` 0)))
    (bind _rootcomponent (`Actor.RootComponent` _asvr_pawn))
    (bind _returnvalue_2 (`SceneComponent.K2_GetComponentLocation` _rootcomponent))
    (bind (_outhit _returnvalue_3) (`KismetSystemLibrary.LineTraceSingleForObjects` :`Start` _returnvalue_2 :`End` (+ _returnvalue_2 (* (`SceneComponent.GetForwardVector` _rootcomponent) 500.0)) :`ObjectTypes` (`|MakeArray` "ObjectTypeQuery2" :!type "EObjectTypeQuery Enum") :`bIgnoreSelf` false))
    (if _returnvalue_3
      (bind _asstatic_mesh_component (cast `StaticMeshComponent` (`.HitComponent` (`GameplayStatics.BreakHitResult` _outhit))))
      (set `self.Static mesh REF` _asstatic_mesh_component)
      (bind _relativelocation_x_3 (`KismetMathLibrary.BreakVector` (`SceneComponent.RelativeLocation` _asstatic_mesh_component)))
      (if (not (>= _relativelocation_x_3 30.0))
        (`GameplayStatics.PlaySoundAtLocation` "/Engine/VREditor/Sounds/UI/Camera_Shutter.Camera_Shutter" _returnvalue (struct) 1.0 1.0 0.0 null null null)
        (set `self.Start location` (`KismetMathLibrary.MakeVector` _relativelocation_x _relativelocation_y _relativelocation_z))
        (set `self.End location` (`KismetMathLibrary.MakeVector` (+ _relativelocation_x 30.0) _relativelocation_y _relativelocation_z))
        (bind (_direction _open_drawer) (`Timeline|open Drawer` :!via `PlayFromStart`)
          (:`Update`
            (`SceneComponent.K2_SetRelativeLocation` (`self.Static mesh REF`) (0.0 0.0 0.0) false false))
          (:`Finished`
            (set `self.can open?` true)))
        (else
          (`GameplayStatics.PlaySoundAtLocation` null _returnvalue (struct) 1.0 1.0 0.0 null null null)
          (set `self.Start location` (`KismetMathLibrary.MakeVector` _relativelocation_x_2 _relativelocation_y_2 _relativelocation_z_2))
          (set `self.End location` (`KismetMathLibrary.MakeVector` (- _relativelocation_x_2 30.0) _relativelocation_y_2 _relativelocation_z_2))
          (bind (_direction_2 _open_drawer_2) (`Timeline|Timeline_0` :!via `PlayFromStart`)
            (:`Update`
              (`SceneComponent.K2_SetRelativeLocation` (`self.Static mesh REF`) (0.0 0.0 0.0) false false))))))))

(fn `UserConstructionScript`)