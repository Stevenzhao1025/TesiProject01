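; Cube Blueprint that changes the opacity of a group of meshes when a box trigger is overlapped, named as a disappear effect.
; Any overlap on the Box plays a timeline whose Xiaoshi track drives the "opacity" scalar material parameter on six static mesh components.
; The construction script creates a dynamic material instance on the first material slot of StaticMeshComponent.
; Nothing reverses the timeline or filters the overlapping actor.
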(event `self.Box.OnComponentBeginOverlap`
  (params (OverlappedComponent :type "PrimitiveComponent Object Reference") (OtherActor :type "Actor Object Reference") (OtherComp :type "PrimitiveComponent Object Reference") (OtherBodyIndex :type Integer) (bFromSweep :type Boolean) (SweepResult :type "HitResult Structure (by ref)"))
  (bind (_direction _xiaoshi) (`Timeline|时间轴_0`)
    (:`Update`
      (`MeshComponent.SetScalarParameterValueOnMaterials` (`self.StaticMesh`) "opacity" _xiaoshi)
      (`MeshComponent.SetScalarParameterValueOnMaterials` (`self.StaticMesh1`) "opacity" _xiaoshi)
      (`MeshComponent.SetScalarParameterValueOnMaterials` (`self.StaticMesh2`) "opacity" _xiaoshi)
      (`MeshComponent.SetScalarParameterValueOnMaterials` (`self.StaticMesh4`) "opacity" _xiaoshi)
      (`MeshComponent.SetScalarParameterValueOnMaterials` (`self.StaticMesh3`) "opacity" _xiaoshi)
      (`MeshComponent.SetScalarParameterValueOnMaterials` (`self.StaticMesh5`) "opacity" _xiaoshi))))

(fn `UserConstructionScript`
  (`PrimitiveComponent.CreateDynamicMaterialInstance` (`self.StaticMeshComponent`) 0 null "None"))