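; VR drawer Blueprint whose static mesh slides along a straight track, following a stored motion controller.
; Each tick, while that controller is valid, the mesh moves to the closest point to it on the segment between the first two spline points.
; As wired, Release stores the controller and Grab clears it if it matches, the reverse of what the event names suggest.
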(event `/Game/blueprint/Grab.Release`
  (params (MotionController :type "MotionControllerComponent Object Reference"))
  (set `self.Motion Controller` MotionController))

(event `/Game/blueprint/Grab.Grab`
  (params (MotionController :type "MotionControllerComponent Object Reference"))
  (if (== MotionController (`self.Motion Controller`))
    (set `self.Motion Controller` null)))

(event `self.ReceiveTick`
  (params (DeltaSeconds :type "Float (single-precision)"))
  (bind _spline (`self.Spline`))
  (bind _motion_controller (`self.Motion Controller`)
    (:`then`
      (`SceneComponent.K2_SetWorldLocation` (`self.StaticMesh`) (`KismetMathLibrary.FindClosestPointOnSegment` (`SceneComponent.K2_GetComponentLocation` _motion_controller) (`SplineComponent.GetLocationAtSplinePoint` _spline 0 "World") (`SplineComponent.GetLocationAtSplinePoint` _spline 1 "World")) false false))
    (:`else`)))

(fn `UserConstructionScript`)