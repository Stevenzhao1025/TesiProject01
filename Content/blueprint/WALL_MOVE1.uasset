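; WALL_MOVE1 is a one-shot triggered wall that slides along its relative X axis when anything overlaps its Box.
; The first overlap passes a DoOnce that is never reset, stores the Wall's current X and plays the 躲开 ("dodge") timeline.
; The timeline track lerps X from that start to start plus Distance, with relative Y and Z left at the setter's defaults.
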(event `self.Box.OnComponentBeginOverlap`
  (params (OverlappedComponent :type "PrimitiveComponent Object Reference") (OtherActor :type "Actor Object Reference") (OtherComp :type "PrimitiveComponent Object Reference") (OtherBodyIndex :type Integer) (bFromSweep :type Boolean) (SweepResult :type "HitResult Structure (by ref)"))
  (bind _wall (`self.wall`))
  (bind _relativelocation_x (`KismetMathLibrary.BreakVector` (`SceneComponent.RelativeLocation` _wall)))
  (`/Engine/EditorBlueprintResources/StandardMacros.DoOnce` false
    (:`Completed`
      (set `self.X` _relativelocation_x)
      (bind (_direction _newtrack_0) (`Timeline|躲开`)
        (:`Update`
          (`SceneComponent.K2_SetRelativeLocation` _wall (`KismetMathLibrary.MakeVector` (`KismetMathLibrary.Lerp` (`self.X`) (+ (`self.X`) (`self.distance`)) _newtrack_0)) false false))))))

(fn `UserConstructionScript`)